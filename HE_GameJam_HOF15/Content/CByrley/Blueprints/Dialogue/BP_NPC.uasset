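; BP_NPC is an idle-animated NPC that shows a text prompt while the player is nearby and stages dialogue scenes with them.
; ActivateDialogue locks movement, enables UI input and adds a black-screen widget, then a timer moves the player to the Cone marker and switches view to the NPC's dialogue camera.
; ExitDialogue returns view to the player camera and restores game input after a delay; result handling is empty.
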(event OnComponentBeginOverlap(SpeakingDistance)
  (params (OverlappedComponent :type Primitive%20Component%20Object%20Reference) (OtherActor :type Actor%20Object%20Reference) (OtherComp :type Primitive%20Component%20Object%20Reference) (OtherBodyIndex :type Integer) (bFromSweep :type Boolean) (SweepResult :type Hit%20Result%20Structure%20%28by%20ref%29))
  (if (CallFunction|IsPlayer OtherActor)
    (Development|SetHiddeninGame (Variables|Default|GetTextRender) false false)))

(event OnComponentEndOverlap(SpeakingDistance)
  (params (OverlappedComponent :type Primitive%20Component%20Object%20Reference) (OtherActor :type Actor%20Object%20Reference) (OtherComp :type Primitive%20Component%20Object%20Reference) (OtherBodyIndex :type Integer))
  (if (CallFunction|IsPlayer OtherActor)
    (Development|SetHiddeninGame (Variables|Default|GetTextRender) true false)))

(event EventBeginPlay
  (Components|Animation|PlayAnimation (Variables|Character|GetMesh) "/Game/Characters/MickeyMouse/Breathing_Idle_Anim.Breathing_Idle_Anim" true))

(event EventActivateDialogue
  (CallFunction|PrepareforDialogue)
  (CallFunction|FadetoBlack))

(event EventExitDialogue
  (params (DialogueReslut :type E_ReplyResult%20Enum :default "NewEnumerator0"))
  (CallFunction|EndDIalogue DialogueReslut))

(fn ConstructionScript
  (Transformation|SetRelativeTransform (Variables|Default|GetDialogueCamera) (Variables|Default|GetCameraTransform) false false)
  (Transformation|SetRelativeLocation (Variables|Default|GetCone) (Variables|Default|GetPlayerLocation) false false))

(fn PrepareforDialogue
  (bind _returnvalue (Game|GetPlayerController 0))
  (Input|SetInputModeUIOnly _returnvalue 0 "DoNotLock" false)
  (Variables|/Script/Engine.PlayerController|SetbShowMouseCursor _returnvalue true)
  (Pawn|Components|CharacterMovement|DisableMovement (Variables|/Script/Engine.Character|GetCharacterMovement (Game|GetPlayerCharacter 0))))

(fn FadetoBlack
  (bind _returnvalue (UserInterface|CreateWidget "/Game/CByrley/Blueprints/Dialogue/WBP_BlackScreen.WBP_BlackScreen_C"))
  (bind _output_get (Variables|Default|SetBlackScreenUIRef _returnvalue))
  (UserInterface|Viewport|AddtoViewport _output_get 0)
  (Utilities|Time|SetTimerbyFunctionName 0 "TeleportPlayerAndCameraToDIaloguePositions" (Variables|Default|GetFadeInAndOUtDuration)))

(fn TeleportPlayerandCameratoDIaloguePositions
  (Game|Player|SetViewTargetwithBlend (Game|GetPlayerController 0) (Components|GetOwner (Variables|Default|GetDialogueCamera)) 0.0 "VTBlend_Linear" 0.0 false)
  (Transformation|SetWorldTransform (Variables|/Script/Engine.Actor|GetRootComponent (Game|GetPlayerCharacter 0)) (Math|Transform|MakeTransform (CallFunction|GetPlayerDIalogueLocation) (CallFunction|GetPlayerDialogueRotation) "1.000000,1.000000,1.000000") false false)
  (Development|SetHiddeninGame (Variables|Default|GetTextRender) true false))

(fn GetPlayerDIalogueLocation
  (bind _cone (Variables|Default|GetCone))
  (bind _returnvalue (Transformation|GetWorldLocation _cone))
  (return (Math|Vector|MakeVector (.x _returnvalue) (.y _returnvalue) (.z (Transformation|GetWorldLocation (Variables|/Script/Engine.Actor|GetRootComponent (Game|GetPlayerCharacter 0)))))))

(fn GetPlayerDialogueRotation
  (bind _returnvalue (Game|GetPlayerCharacter 0))
  (bind _rootcomponent (Variables|/Script/Engine.Actor|GetRootComponent _returnvalue))
  (bind _returnvalue_2 (Transformation|GetWorldRotation _rootcomponent))
  (return (Math|Rotator|MakeRotator (.roll _returnvalue_2) (.pitch _returnvalue_2) (+ (.yaw (Transformation|GetWorldRotation (Variables|Character|GetMesh))) -9e+01))))

(fn EndDIalogue
  (params (DialogueResult :type E_ReplyResult%20Enum :default "NewEnumerator0"))
  (CallFunction|TRansitionOutOfDialogue)
  (if (Utilities|Enum|Equal(Enum) DialogueResult "NewEnumerator2")
    _))

(fn TRansitionOutOfDialogue
  (bind _asbp_player_character (Utilities|Casting|CastToBP_PlayerCharacter (Game|GetPlayerCharacter 0)))
  (Game|Player|SetViewTargetwithBlend (Game|GetPlayerController 0) (Components|GetOwner (Variables|/Game/TylerM/PlayerCharacter/BP_PlayerCharacter.BP_PlayerCharacter_C|GetCamera _asbp_player_character)) 0.0 "VTBlend_Linear" (Variables|Default|GetTransitionOutDuration) false)
  (Variables|/Script/Engine.PlayerController|SetbShowMouseCursor (Game|GetPlayerController 0) false)
  (Utilities|Time|SetTimerbyFunctionName 0 "ResumePlayerGameInput" (Variables|Default|GetTransitionOutDuration)))

(fn ResumePlayerGameInput
  (Input|SetInputModeGameOnly (Game|GetPlayerController 0) false)
  (Pawn|Components|CharacterMovement|SetMovementMode (Variables|/Script/Engine.Character|GetCharacterMovement (Game|GetPlayerCharacter 0)) "MOVE_Walking" 0))

(fn GetNPCName
  (return (Utilities|Text|ToText(String) (Variables|Default|GetNPCName))))