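; Zombie enemy character that chases the player, attacks in melee and dies when damaged.
; Pawn sensing triggers AIMoveTo toward the player, and reaching them plays an attack montage gated by CanAttack for its duration.
; A sphere overlap damages BP_PlayerCharacter only during an attack.
; Any damage is passed to ACHealth but always starts death, blocking new chases and destroying the actor after the dying montage.
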(event OnSeePawn(PawnSensing)
  (params (Pawn :type Pawn%20Object%20Reference))
  (Variables|Default|SetIsSeeingPlayer true)
  (CallFunction|FollowPlayer))

(event OnComponentBeginOverlap(Sphere)
  (params (OverlappedComponent :type Primitive%20Component%20Object%20Reference) (OtherActor :type Actor%20Object%20Reference) (OtherComp :type Primitive%20Component%20Object%20Reference) (OtherBodyIndex :type Integer) (bFromSweep :type Boolean) (SweepResult :type Hit%20Result%20Structure%20%28by%20ref%29))
  (bind _asbp_player_character (Utilities|Casting|CastToBP_PlayerCharacter OtherActor))
  (if (Variables|Default|GetIsAttacking)
    (bind _returnvalue (Game|Damage|ApplyDamage _asbp_player_character 5e+01 0 0))
    (Development|PrintString (Utilities|String|ToString(Float) _returnvalue))))

(event Custom|FollowPlayer
  (if (not (Variables|Default|GetIsDying?))
    (AI|AIMoveTo self "0, 0, 0" (Game|GetPlayerCharacter 0) 35.0 false
      (:OnSuccess
        (if (Variables|Default|GetCanAttack?)
          (Variables|Default|SetCanAttack? false)
          (Variables|Default|SetIsAttacking true)
          (bind _returnvalue (Animation|PlayAnimMontage "/Game/Characters/BloodyMickyMouse/Animations/Zombie_Attack__1__Montage.Zombie_Attack__1__Montage" 1.0 "None"))
          (Utilities|FlowControl|Delay _returnvalue)
          (Variables|Default|SetCanAttack? true)
          (Variables|Default|SetIsAttacking false))))))

(event EventBeginPlay)

(event Collision|EventActorBeginOverlap
  (params (OtherActor :type Actor%20Object%20Reference)))

(event EventTick
  (params (DeltaSeconds :type Float%20%28single-precision%29)))

(event Game|Damage|EventAnyDamage
  (params (Damage :type Float%20%28single-precision%29) (DamageType :type Damage%20Type%20Object%20Reference) (InstigatedBy :type Controller%20Object%20Reference) (DamageCauser :type Actor%20Object%20Reference))
  (Default|Health (Variables|Default|GetAC_Health) Damage)
  (Variables|Default|SetIsDying? true)
  (bind _returnvalue (Animation|PlayAnimMontage "/Game/Characters/BloodyMickyMouse/Animations/Zombie_Dying_Montage.Zombie_Dying_Montage" 1.3 "None"))
  (Utilities|FlowControl|Delay _returnvalue)
  (Actor|DestroyActor))

(fn ConstructionScript)